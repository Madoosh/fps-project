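; Interactable static mesh actor that fades between visible and hidden when a player interacts, switching its collision profile to match.
; The server steps a delay loop through transitional states, multicasting the clamped opacity to a material scalar parameter until it finishes.
; CollisionAtStart decides whether collision switches as the fade begins or ends.
; A looping half-second timer re-sends settled opacity through a client event to keep visibility in sync.
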(event Custom|Client_ChangeVisibility
  (params (ParameterValue :type Float%20%28single-precision%29))
  ;[1 1 1] Change visibility
  (Rendering|Material|SetScalarParameterValueonMaterials (Variables|Default|GetStaticMesh) (Variables|Settings|More|GetOpacityMatName) (Math|Float|Clamp(Float) ParameterValue (Variables|Settings|More|GetMinimumOpacity) (Variables|Settings|More|GetMaximumOpacity))))

(event Custom|Server_PlayerInteract
  ;[1 1 1] On player interact
  (Networking|SwitchHasAuthority
    (:Authority
      (switch Utilities|FlowControl|Switch|SwitchonE_AntizeVisibility (Variables|Default|GetActualVisibility)
        (:NewEnumerator0
          (Variables|Default|SetActualVisibility "NewEnumerator3"))
        (:NewEnumerator1
          (Variables|Default|SetActualVisibility "NewEnumerator2")))
      (CallFunction|ServerChangeVisibility))))

(event Custom|Server_ChangeVisibility
  (bind _timerspeed (Variables|Settings|GetTimerSpeed))
  ;[1 1 1] Do animation
  (Networking|SwitchHasAuthority
    (:Authority
      (bind _output_get (Variables|Default|SetToVisible? (Utilities|Select :Index (Variables|Default|GetActualVisibility) :NewEnumerator0 true :NewEnumerator1 false :NewEnumerator2 true :NewEnumerator3 false)))
      (Variables|Default|SetActualTimeDo (select _output_get 0.0 (Variables|Settings|GetVisibilityDelay)))
      (Utilities|FlowControl|Sequence
        (:then_0
          (Utilities|FlowControl|Delay (Variables|Settings|GetTimerSpeed) :!label _label)
          (Variables|Default|SetActualTimeDo (select (Variables|Default|GetToVisible?) (+ (Variables|Default|GetActualTimeDo) _timerspeed) (- (Variables|Default|GetActualTimeDo) _timerspeed)))
          (if (select (Variables|Default|GetToVisible?) (>= (Variables|Default|GetActualTimeDo) (Variables|Settings|GetVisibilityDelay)) (<= (Variables|Default|GetActualTimeDo) 0.0))
            (CallFunction|FinishChangeVisibility)
            (else
              (CallFunction|MultiChangeVisibility (/ (Variables|Default|GetActualTimeDo) (Variables|Settings|GetVisibilityDelay)))
              (goto _label))))
        (:then_1
          (if (Variables|Settings|More|GetCollisionAtStart?)
            (Collision|SetCollisionProfileName (Variables|Default|GetStaticMesh) (select (Variables|Default|GetToVisible?) "AntizeInteractTrue" "AntizeInteractFalse") true :!class /Script/Engine.PrimitiveComponent)))))))

(event Custom|FinishChangeVisibility
  ;[1 1 1] Finish animation
  (Networking|SwitchHasAuthority
    (:Authority
      (CallFunction|MultiChangeVisibility (select (Variables|Default|GetToVisible?) (Variables|Settings|More|GetMaximumOpacity) (Variables|Settings|More|GetMinimumOpacity)))
      (Variables|Default|SetActualVisibility (select (Variables|Default|GetToVisible?) "NewEnumerator0" "NewEnumerator1"))
      (if (not (Variables|Settings|More|GetCollisionAtStart?))
        (Collision|SetCollisionProfileName (Variables|Default|GetStaticMesh) (select (Variables|Default|GetToVisible?) "AntizeInteractTrue" "AntizeInteractFalse") true :!class /Script/Engine.PrimitiveComponent)))))

(event Custom|Multi_ChangeVisibility
  (params (ParameterValue :type Float%20%28single-precision%29))
  ;[1 1 1] Change visibility
  (Rendering|Material|SetScalarParameterValueonMaterials (Variables|Default|GetStaticMesh) (Variables|Settings|More|GetOpacityMatName) (Math|Float|Clamp(Float) ParameterValue (Variables|Settings|More|GetMinimumOpacity) (Variables|Settings|More|GetMaximumOpacity))))

(event Custom|ForceCheck
  ;[1 1 1] BeginPlay
  ;;[1 1 1] Be sure to change visibility
  (switch Utilities|FlowControl|Switch|SwitchonE_AntizeVisibility (Variables|Default|GetActualVisibility)
    (:NewEnumerator0
      (CallFunction|ClientChangeVisibility (Variables|Settings|More|GetMaximumOpacity)))
    (:NewEnumerator1
      (CallFunction|ClientChangeVisibility (Variables|Settings|More|GetMinimumOpacity)))))

(event EventBeginPlay
  ;[1 1 1] BeginPlay
  (Utilities|Time|SetTimerbyEvent (delegate Custom|ForceCheck) 0.5 true)
  (Networking|SwitchHasAuthority
    (:Authority
      (switch Utilities|FlowControl|Switch|SwitchonE_AntizeVisibility (Variables|Default|GetActualVisibility)
        (:NewEnumerator0
          (Variables|Default|SetToVisible? true)
          (CallFunction|FinishChangeVisibility :!label _label))
        (:NewEnumerator1
          (Variables|Default|SetToVisible? false)
          (goto _label))
        (:NewEnumerator2
          (CallFunction|ServerChangeVisibility :!label _label_2))
        (:NewEnumerator3
          (goto _label_2))))))

(fn ConstructionScript
  (Components|StaticMesh|SetStaticMesh (Variables|Default|GetStaticMesh) (Variables|Settings|GetMyStaticMesh)))