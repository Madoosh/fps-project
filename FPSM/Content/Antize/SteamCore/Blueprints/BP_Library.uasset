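; BP_Library holds Steam helper functions for lobby membership and friend chat windows in the SteamCore Blueprints.
; IsInLobby loops over a lobby's members and returns true if one matches the local user's Steam ID.
; FindFriendChatWindow searches all WBP_FriendChatWindow widgets, including nested ones, and returns the one whose SteamFriendID matches the given friend.
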(fn IsinLobby
  (params (SteamIDLobby :type Steam%20ID%20Structure))
  (bind _returnvalue (Class|Matchmaking|GetNumLobbyMembers SteamIDLobby))
  (for _index (range 0 (- _returnvalue 1))
    (bind _returnvalue_2 (Class|Matchmaking|GetLobbyMemberbyIndex SteamIDLobby _index))
    (if (Class|SteamUtilities|Equal _returnvalue_2 (Class|User|GetSteamIDPure))
      (return true)))
  (return false))

(fn FindFriendChatWindow
  (params (SteamFriendID :type Steam%20ID%20Structure))
  (bind _foundwidgets (Widget|GetAllWidgetsOfClass 0 "/Game/Antize/SteamCore/Blueprints/UMG/Friends/WBP_FriendChatWindow.WBP_FriendChatWindow_C" false))
  (for _array_element _foundwidgets
    (if (Class|SteamUtilities|Equal (Variables|/Game/Antize/SteamCore/Blueprints/UMG/Friends/WBP_FriendChatWindow.WBP_FriendChatWindow_C|GetSteamFriendID _array_element) SteamFriendID)
      (return _array_element))))