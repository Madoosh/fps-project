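; BP_LampInteract is an interactable lamp that the player can switch on and off.
; OnInteract, triggered from the controller, flips ActualOn, applies it to the PointLight's visibility and calls UpdateActionText.
; It also sets the Color parameter on MaterialRef to red when on and white when off.
; The construction script only calls its parent, and BeginPlay is disabled.
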(event EventBeginPlay
  (|CallParentFunction) ; This node is disabled and will not be called.\nDrag off pins to build functionality.
)

(event EventOnInteract
  ;[1 1 1] Interact (From Controller)
  (if (Variables|Default|GetActualOn?)
    (Variables|Default|SetActualOn? false)
    (else
      (Variables|Default|SetActualOn? true)))
  (Rendering|SetVisibility (Variables|Default|GetPointLight) (Variables|Default|GetActualOn?) false)
  (CallFunction|UpdateActionText)
  (Rendering|Material|SetVectorParameterValue (Variables|Default|GetMaterialRef) "Color" (select (Variables|Default|GetActualOn?) "(R=1.000000,G=0.000000,B=0.000000,A=1.000000)" "(R=1.000000,G=1.000000,B=1.000000,A=1.000000)") :!class /Script/Engine.MaterialInstanceDynamic))

(fn ConstructionScript
  (|CallParentFunction))