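; Competitive game mode for the Rush mode, managing bombs and staged player spawns.
; On BeginPlay it sets the mode type, gathers spawns, checks game options and adjusts bot count.
; Disabling bombs spares one kept bomb and sends it to every valid player controller as the client Rush marker.
; Spawn activation enables only the A and B spawn points whose State matches the requested one.
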(event Custom|ActivateNewSpawns
  (params (NewParam :type Integer))
  ;[1 1 1] Activate New Spawns
  (for _array_element (Variables|Default|GetPlayerSpawnsA)
    (Variables|/Game/FPS/Blueprints/Misc/PlayerSpawn/BP_PlayerSpawn.BP_PlayerSpawn_C|SetbActive _array_element (== NewParam (Variables|/Game/FPS/Blueprints/Misc/PlayerSpawn/BP_PlayerSpawn.BP_PlayerSpawn_C|GetState _array_element))))
  (for _array_element_2 (Variables|Default|GetPlayerSpawnsB)
    (Variables|/Game/FPS/Blueprints/Misc/PlayerSpawn/BP_PlayerSpawn.BP_PlayerSpawn_C|SetbActive _array_element_2 (== NewParam (Variables|/Game/FPS/Blueprints/Misc/PlayerSpawn/BP_PlayerSpawn.BP_PlayerSpawn_C|GetState _array_element_2)))))

(event Custom|GM_DisableBombe
  (params (KeepRef :type BP%20Bomb%20Object%20Reference))
  (bind _outactors (Actor|GetAllActorsOfClass "/Game/FPS/Blueprints/Interactables/Bomb/BP_Bomb.BP_Bomb_C"))
  (for _array_element _outactors
    (if (!= _array_element KeepRef)
      (Default|ServerDisableBombe _array_element)))
  (for _array_element_2 (Variables|Default|GetAllPlayersPCs)
    (Utilities|IsValid _array_element_2
      (:Is%20Valid
        (bind _asbase_player_controller (Utilities|Casting|CastToBasePlayerController _array_element_2))
        (Default|ClientUpdateRushMarker _asbase_player_controller KeepRef)))))

(event EventBeginPlay
  ;[1 1 1] Begin Play
  (Variables|Default|SetGameMode "NewEnumerator1")
  (CallFunction|GetPlayerSpawns)
  (CallFunction|CheckGameOptions)
  (CallFunction|ManageNumberOfBots))

(fn ConstructionScript
  (|CallParentFunction))